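; Enemy patrol character that chases the player and has BP_GameControl imprison any third-person character it overlaps, whether chasing or not.
; It registers itself with AIC_EnemyPatrol on BeginPlay and provides its patrol route and enum-based walk speed setting.
; ChasePlayer starts tension audio and re-issues AIMoveTo after each successful move and a delay.
; StopChasingPlayer only fades out that audio, without clearing IsChasing or cancelling movement.
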(event `self.ReceiveBeginPlay`
  (bind _asaic_enemy_patrol (cast `/Game/AI/AIC_EnemyPatrol` (`AIBlueprintHelperLibrary.GetAIController` self)))
  (set `/Game/AI/AIC_EnemyPatrol.BP_TestPatrol` self _asaic_enemy_patrol))

(event `ChasePlayer`
  ;[1 1 1] Chasing Function
  (set `self.IsChasing` true)
  (if (not (`KismetSystemLibrary.IsValid` (`self.ChasingSound`)))
    (bind _returnvalue (`GameplayStatics.SpawnSound2D` "/Game/Sounds/Enemy/ChasingTension_Cue.ChasingTension_Cue" 1.0 1.0 0.0 null false false))
    (set `self.ChasingSound` _returnvalue)
    (`KismetSystemLibrary.Delay` 0.2))
  (`|AIMoveTo` self (0.0 0.0 0.0) (`GameplayStatics.GetPlayerCharacter` 0) 150.0
    (:`OnSuccess`
      (`KismetSystemLibrary.Delay` 2.0)
      (`self.ChasePlayer`))))

(event `StopChasingPlayer`
  (bind _chasingsound (`self.ChasingSound`))
  ;[1 1 1] Chasing Function
  (`/Engine/EditorBlueprintResources/StandardMacros.IsValid` _chasingsound
    (:`Is Valid`
      (`AudioComponent.FadeOut` _chasingsound 0.5 0.0 "Linear")
      (set `self.ChasingSound` null))))

(event `self.ReceiveActorBeginOverlap`
  (params (OtherActor :type "Actor Object Reference"))
  ;[1 1 1] TODO: MAKE IT SO THAT THE CAPTURE HAPPENS ONLY WHEN THE ACTOR IS CHASING PLAYER?
  (bind _asbp_third_person_character (cast `/Game/Prototype/Blueprints/ThirdPersonCharacter/BP_ThirdPersonCharacter` OtherActor))
  (bind _returnvalue (`GameplayStatics.GetActorOfClass` "/Game/Prototype/Blueprints/GameControl/BP_GameControl.BP_GameControl_C"))
  (`/Game/Prototype/Blueprints/GameControl/BP_GameControl.Imprison Player` _returnvalue _asbp_third_person_character self))

(fn `GetPatrolRoute`
  (returns (PatrolRoute :type "/Game/AI/BP_PatrolRoute Object Reference"))
  (return (`self.PatrolRoute`)))

(fn `SetMovementSpeed`
  (params (Speed :type "/Game/AI/Enums/E_MovementSpeed Enum" :default "NewEnumerator0"))
  (returns (SpeedValue :type "Float (double-precision)"))
  (bind _output_get (set `CharacterMovementComponent.MaxWalkSpeed` (select `/Game/AI/Enums/E_MovementSpeed` Speed :`NewEnumerator1` 100.0 :`NewEnumerator2` 300.0 :`NewEnumerator3` 400.0 :!type "Float (single-precision)") (`self.CharacterMovement`)))
  (return _output_get))

(fn `UserConstructionScript`)