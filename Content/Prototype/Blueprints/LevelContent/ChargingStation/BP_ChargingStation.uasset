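; BP_ChargingStation recharges the battery of a BP_ThirdPersonCharacter while that player overlaps it.
; Overlap events set the charging state on both station and player, and Tick calls the player's ChargeBattery.
; If Overloads is enabled, delivered charge accumulates until a warning threshold resets it and calls DoOverload.
; DoOverload makes AI noise at the player's location, plays an alarm sound and triggers the child-actor BP_AlarmLight.
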(event `self.ReceiveTick`
  (params (DeltaSeconds :type "Float (single-precision)"))
  (if (`self.Is Charging`)
    (bind _recharged_amount (`/Game/Prototype/Blueprints/ThirdPersonCharacter/BP_ThirdPersonCharacter.Charge Battery` (`self.Player Being Charged`) (`self.Charge Speed`) DeltaSeconds))
    (if (`self.Overloads`)
      (bind _output_get (set `self.Current Charge Threshold` (+ _recharged_amount (`self.Current Charge Threshold`))))
      (if (>= _output_get (`self.Charge Warning Threshold`))
        (set `self.Current Charge Threshold` 0.0)
        (`self.Do Overload`)))))

(event `self.ReceiveActorBeginOverlap`
  (params (OtherActor :type "Actor Object Reference"))
  (bind _asbp_third_person_character (cast `/Game/Prototype/Blueprints/ThirdPersonCharacter/BP_ThirdPersonCharacter` OtherActor))
  (bind _output_get (set `self.Player Being Charged` _asbp_third_person_character))
  (set `/Game/Prototype/Blueprints/ThirdPersonCharacter/BP_ThirdPersonCharacter.Is Recharging` true _output_get)
  (set `self.Is Charging` true))

(event `self.ReceiveActorEndOverlap`
  (params (OtherActor :type "Actor Object Reference"))
  (bind _asbp_third_person_character (cast `/Game/Prototype/Blueprints/ThirdPersonCharacter/BP_ThirdPersonCharacter` OtherActor))
  (set `/Game/Prototype/Blueprints/ThirdPersonCharacter/BP_ThirdPersonCharacter.Is Recharging` false _asbp_third_person_character)
  (set `self.Player Being Charged` null)
  (set `self.Is Charging` false))

(fn `Do Overload`
  (bind _returnvalue (`GameplayStatics.GetActorOfClass` "/Game/Prototype/Blueprints/ThirdPersonCharacter/BP_ThirdPersonCharacter.BP_ThirdPersonCharacter_C"))
  (`self.MakeNoise` 1.0 _returnvalue (`self.K2_GetActorLocation` _returnvalue))
  (`GameplayStatics.PlaySoundAtLocation` "/Game/Sounds/Environment/Alarm_Triggered.Alarm_Triggered" (`self.K2_GetActorLocation`) (struct) 0.5 1.0 0.0 null null null null)
  (bind _asbp_alarm_light (cast `/Game/Prototype/Blueprints/LevelContent/ChargingStation/BP_AlarmLight` (`ChildActorComponent.ChildActor` (`self.BP_AlarmLight`))))
  (`/Game/Prototype/Blueprints/LevelContent/ChargingStation/BP_AlarmLight.Trigger Alarm` _asbp_alarm_light))

(fn `UserConstructionScript`)