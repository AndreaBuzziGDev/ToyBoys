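; BP_AlarmLight is an alarm light in the charging station level content that pulses for a set duration when triggered.
; TriggerAlarm shows the initially hidden point light, resets the timer and arms the effect.
; While triggered, Tick advances the timer and drives intensity with an absolute cosine wave scaled by frequency, maximum and minimum intensity values.
; Once the alarm duration elapses, it resets and hides the light again.
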(event `self.ReceiveBeginPlay`
  (`SceneComponent.SetHiddenInGame` (`self.PointLight`) true true))

(event `self.ReceiveTick`
  (params (DeltaSeconds :type "Float (single-precision)"))
  (if (`self.Is Triggered`)
    (`self.Handle Light Intensity Change` DeltaSeconds)))

(fn `Handle Light Intensity Change`
  (params (`Delta Seconds` :type "Float (double-precision)"))
  (bind _output_get (set `self.Elapsed Time` (+ (`self.Elapsed Time`) `Delta Seconds`)))
  (`LightComponent.SetIntensity` (`self.PointLight`) (+ (* (`KismetMathLibrary.Abs` (`KismetMathLibrary.Cos` (* _output_get (`self.Frequency`)))) (`self.Max Intensity`)) (`self.Min Intensity`)))
  (if (>= (`self.Elapsed Time`) (`self.Alarm Duration`))
    (set `self.Elapsed Time` 0.0)
    (set `self.Is Triggered` false)
    (`SceneComponent.SetHiddenInGame` (`self.PointLight`) true true)))

(fn `Trigger Alarm`
  (`SceneComponent.SetHiddenInGame` (`self.PointLight`) false true)
  (set `self.Elapsed Time` 0.0)
  (set `self.Is Triggered` true))

(fn `UserConstructionScript`)