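; Interactable resource actor that acts as a bypass for alarms in the level.
; Installing the resource unhides its scene component and all children in game, then runs the parent install logic.
; On an activation signal it flags every associated alarm as bypassed before passing the signal to the parent class.
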(fn `Install Resource`
  (`SceneComponent.SetHiddenInGame` (`self.My Scene`) false true)
  (`parent.Install Resource`))

(fn `Receive Activation Signal`
  (for _array_element (`self.Associated Alarms`)
    (set `/Game/Prototype/Blueprints/LevelContent/ChargingStation/BP_ChargingStation_Overloading.Is Bypassed` true _array_element))
  (`parent.Receive Activation Signal`))

(fn `UserConstructionScript`
  (`parent.UserConstructionScript`))