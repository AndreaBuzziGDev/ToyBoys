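; Template Blueprint for a pickup interactable that players can target when in range.
; On BeginPlay it passes itself to its BigArm interaction prompt child actor as that prompt's owning interactable.
; SetPlayerInteractability sets or clears the player's OverlappingPickable reference and shows or hides a debug light.
; The PickUp function and construction script are empty stubs.
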(event `self.ReceiveBeginPlay`
  (bind _asbp_interaction_prompt_big_arm (cast `/Game/Prototype/Blueprints/LevelContent/InteractableObjects/Interactions/DoNotUse/Interactable_Object_Prompt/BP_Interaction_Prompt_BigArm` (`ChildActorComponent.ChildActor` (`self.BP_Interaction_Prompt_BigArm`))))
  (set `/Game/Prototype/Blueprints/LevelContent/InteractableObjects/Interactions/DoNotUse/Interactable_Object_Prompt/Technical/BP_Interaction_Prompt_Generic.My Own Interactable` self _asbp_interaction_prompt_big_arm))

(fn `Pick Up`)

(fn `Set Player Interactability`
  (params (`Is Interactable` :type Boolean) (`Affected Player` :type "/Game/Prototype/Blueprints/ThirdPersonCharacter/BP_ThirdPersonCharacter Object Reference"))
  (bind _debug_light (`self.Debug Light`))
  ;[1 1 1] Comment
  (if `Is Interactable`
    (set `/Game/Prototype/Blueprints/ThirdPersonCharacter/BP_ThirdPersonCharacter.Overlapping Pickable` self `Affected Player`)
    (`SceneComponent.SetHiddenInGame` _debug_light false true)
    (else
      (set `/Game/Prototype/Blueprints/ThirdPersonCharacter/BP_ThirdPersonCharacter.Overlapping Pickable` null `Affected Player`)
      (`SceneComponent.SetHiddenInGame` _debug_light true true))))

(fn `UserConstructionScript`)