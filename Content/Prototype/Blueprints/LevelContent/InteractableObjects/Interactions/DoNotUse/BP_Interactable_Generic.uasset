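; Generic interactable base actor that pairs a physics mesh with a child-actor interaction prompt, registering itself with that prompt on BeginPlay.
; SetPlayerInteractability toggles a debug light as a placeholder highlight, hides the light on the player's previous OverlappingPickable, and calls SetOverlappingProperty, an empty hook here.
; Enable and Disable toggle visibility, tick, mesh physics and collision, and the prompt's detection box, with Disable also hiding the prompt.
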(event `self.ReceiveBeginPlay`
  (bind _asbp_interaction_prompt_generic (cast `/Game/Prototype/Blueprints/LevelContent/InteractableObjects/Interactions/DoNotUse/Interactable_Object_Prompt/Technical/BP_Interaction_Prompt_Generic` (`ChildActorComponent.ChildActor` (`self.BP_Interaction_Prompt_Generic`))))
  (set `/Game/Prototype/Blueprints/LevelContent/InteractableObjects/Interactions/DoNotUse/Interactable_Object_Prompt/Technical/BP_Interaction_Prompt_Generic.My Own Interactable` self _asbp_interaction_prompt_generic))

(fn `Disable`
  (bind _my_static_mesh (`self.My Static Mesh`))
  (bind _asbp_interaction_prompt_generic (cast `/Game/Prototype/Blueprints/LevelContent/InteractableObjects/Interactions/DoNotUse/Interactable_Object_Prompt/Technical/BP_Interaction_Prompt_Generic` (`ChildActorComponent.ChildActor` (`self.BP_Interaction_Prompt_Generic`))))
  (`/Game/Prototype/Blueprints/LevelContent/InteractableObjects/Interactions/DoNotUse/Interactable_Object_Prompt/Technical/BP_Interaction_Prompt_Generic.Handle Prompt Show` _asbp_interaction_prompt_generic false)
  (`PrimitiveComponent.SetCollisionEnabled` (`/Game/Prototype/Blueprints/LevelContent/InteractableObjects/Interactions/DoNotUse/Interactable_Object_Prompt/Technical/BP_Interaction_Prompt_Generic.Player Detection Box` _asbp_interaction_prompt_generic) "NoCollision")
  (`self.SetActorHiddenInGame` true)
  (`self.SetActorTickEnabled` false)
  (`PrimitiveComponent.SetSimulatePhysics` _my_static_mesh false)
  (`PrimitiveComponent.SetCollisionEnabled` _my_static_mesh "NoCollision"))

(fn `Enable`
  (bind _my_static_mesh (`self.My Static Mesh`))
  (`self.SetActorHiddenInGame` false)
  (`self.SetActorTickEnabled` true)
  (`PrimitiveComponent.SetSimulatePhysics` _my_static_mesh true)
  (`PrimitiveComponent.SetCollisionEnabled` _my_static_mesh "QueryAndPhysics")
  (bind _asbp_interaction_prompt_generic (cast `/Game/Prototype/Blueprints/LevelContent/InteractableObjects/Interactions/DoNotUse/Interactable_Object_Prompt/Technical/BP_Interaction_Prompt_Generic` (`ChildActorComponent.ChildActor` (`self.BP_Interaction_Prompt_Generic`))))
  (`PrimitiveComponent.SetCollisionEnabled` (`/Game/Prototype/Blueprints/LevelContent/InteractableObjects/Interactions/DoNotUse/Interactable_Object_Prompt/Technical/BP_Interaction_Prompt_Generic.Player Detection Box` _asbp_interaction_prompt_generic) "QueryOnly"))

(fn `Set Overlapping Property`
  (params (`Affected Interactable` :type "/Game/Prototype/Blueprints/LevelContent/InteractableObjects/Interactions/DoNotUse/BP_Interactable_Generic Object Reference") (`Affected Player` :type "/Game/Prototype/Blueprints/ThirdPersonCharacter/BP_ThirdPersonCharacter Object Reference")))

(fn `Set Player Interactability`
  (params (`Is Interactable` :type Boolean) (`Affected Player` :type "/Game/Prototype/Blueprints/ThirdPersonCharacter/BP_ThirdPersonCharacter Object Reference"))
  (bind _overlapping_pickable (`/Game/Prototype/Blueprints/ThirdPersonCharacter/BP_ThirdPersonCharacter.Overlapping Pickable` `Affected Player`))
  (bind _debug_light (`self.Debug Light`))
  ;[1 1 1] TODO: This should evolve and change the material or do something of that kind to mark an interactable pickup
  (if `Is Interactable`
    (`/Engine/EditorBlueprintResources/StandardMacros.IsValid` _overlapping_pickable
      (:`Is Valid`
        (`SceneComponent.SetHiddenInGame` (`/Game/Prototype/Blueprints/LevelContent/InteractableObjects/Interactions/DoNotUse/BP_Interactable_Generic.Debug Light` _overlapping_pickable) true true))
      (:`Is Not Valid`
        _))
    (`self.Set Overlapping Property` self `Affected Player`)
    (`SceneComponent.SetHiddenInGame` _debug_light false true)
    (else
      (`self.Set Overlapping Property` null `Affected Player`)
      (`SceneComponent.SetHiddenInGame` _debug_light true true))))

(fn `UserConstructionScript`)