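; Template interactable that acts as a clearance gate, pushing away third-person characters who lack the required module.
; When a character overlaps its mesh, it maps the prompt type of its child interaction prompt through ClearanceMapping and compares the result with the character's SceneHead module.
; On a mismatch, Repel applies a velocity-change impulse away from the actor, with separate horizontal and vertical strengths.
; SetOverlappingProperty is left empty.
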(event `self.My Static Mesh.OnComponentBeginOverlap`
  (params (OverlappedComponent :type "PrimitiveComponent Object Reference") (OtherActor :type "Actor Object Reference") (OtherComp :type "PrimitiveComponent Object Reference") (OtherBodyIndex :type Integer) (bFromSweep :type Boolean) (SweepResult :type "HitResult Structure (by ref)"))
  (bind _asbp_third_person_character (cast `/Game/Prototype/Blueprints/ThirdPersonCharacter/BP_ThirdPersonCharacter` OtherActor))
  (bind _has_clearance (`self.Check Clearance` _asbp_third_person_character))
  (if (not _has_clearance)
    (`self.Repel` _asbp_third_person_character)))

(fn `Check Clearance`
  (params (Player :type "/Game/Prototype/Blueprints/ThirdPersonCharacter/BP_ThirdPersonCharacter Object Reference"))
  (returns (`Has Clearance` :type Boolean))
  (bind _asbp_interaction_prompt_generic (cast `/Game/Prototype/Blueprints/LevelContent/InteractableObjects/Interactions/DoNotUse/Interactable_Object_Prompt/Technical/BP_Interaction_Prompt_Generic` (`ChildActorComponent.ChildActor` (`self.BP_Interaction_Prompt_Generic`))))
  (bind _asbp_scene_head (cast `/Game/Prototype/Blueprints/ModularSystem/PlayerModules/ThirdPersonCharacterSceneModules/BP_SceneHead` (`ChildActorComponent.ChildActor` (`/Game/Prototype/Blueprints/ThirdPersonCharacter/BP_ThirdPersonCharacter.BP_SceneHead` Player))))
  (return (`|EnumEquality` (`BlueprintMapLibrary.Map_Find` (`self.Clearance Mapping`) (`/Game/Prototype/Blueprints/LevelContent/InteractableObjects/Interactions/DoNotUse/Interactable_Object_Prompt/Technical/BP_Interaction_Prompt_Generic.Prompt Type` _asbp_interaction_prompt_generic)) (`/Game/Prototype/Blueprints/ModularSystem/PlayerModules/ThirdPersonCharacterSceneModules/BP_SceneHead.Module` _asbp_scene_head))))

(fn `Repel`
  (params (Player :type "/Game/Prototype/Blueprints/ThirdPersonCharacter/BP_ThirdPersonCharacter Object Reference"))
  (`CharacterMovementComponent.AddImpulse` (`Character.CharacterMovement` Player) (`KismetMathLibrary.MakeVector` (* (.x (`KismetMathLibrary.Normal` (- (`self.K2_GetActorLocation` Player) (`self.K2_GetActorLocation`)))) (`self.Repulsion Strength Horizontal`)) (* (.y (`KismetMathLibrary.Normal` (- (`self.K2_GetActorLocation` Player) (`self.K2_GetActorLocation`)))) (`self.Repulsion Strength Horizontal`)) (* (.z (`KismetMathLibrary.Normal` (- (`self.K2_GetActorLocation` Player) (`self.K2_GetActorLocation`)))) (`self.Repulsion Strength Vertical`))) true))

(fn `Set Overlapping Property`
  (params (`Affected Interactable` :type "/Game/Prototype/Blueprints/LevelContent/InteractableObjects/Interactions/DoNotUse/BP_Interactable_Generic Object Reference") (`Affected Player` :type "/Game/Prototype/Blueprints/ThirdPersonCharacter/BP_ThirdPersonCharacter Object Reference")))

(fn `UserConstructionScript`
  (`parent.UserConstructionScript`))