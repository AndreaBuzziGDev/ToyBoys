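; BP_FanTeleport is an activatable level object that teleports the player character when it enters the box trigger while the teleporter is active.
; Activate switches it on through the parent logic, and a repeat call switches it off only if it is deactivable.
; The character moves to the location and rotation of the associated destination's TeleportPosition, or a message prints when no destination is set.
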(event `self.Box.OnComponentBeginOverlap`
  (params (OverlappedComponent :type "PrimitiveComponent Object Reference") (OtherActor :type "Actor Object Reference") (OtherComp :type "PrimitiveComponent Object Reference") (OtherBodyIndex :type Integer) (bFromSweep :type Boolean) (SweepResult :type "HitResult Structure (by ref)"))
  (bind _asbp_third_person_character (cast `/Game/Prototype/Blueprints/ThirdPersonCharacter/BP_ThirdPersonCharacter` OtherActor))
  (if (`self.Is Active`)
    (`self.Teleport player` _asbp_third_person_character)))

(fn `Activate`
  (bind _is_active (`self.Is Active`))
  (if _is_active
    (if (`self.Is Deactivable`)
      (set `self.Is Active` (not _is_active)))
    (else
      (set `self.Is Active` true)
      (`parent.Activate`))))

(fn `Teleport player`
  (params (`Teleported Player` :type "/Game/Prototype/Blueprints/ThirdPersonCharacter/BP_ThirdPersonCharacter Object Reference"))
  (bind _associated_teleport_destination (`self.Associated Teleport Destination`))
  (`/Engine/EditorBlueprintResources/StandardMacros.IsValid` _associated_teleport_destination
    (:`Is Valid`
      (`self.K2_SetActorLocationAndRotation` `Teleported Player` (.location (`SceneComponent.K2_GetComponentToWorld` (`/Game/Prototype/Blueprints/LevelContent/InteractableObjects/Interactions/Activable/Utilities/BP_TeleportDestination.Teleport Position` _associated_teleport_destination))) (.rotation (`SceneComponent.K2_GetComponentToWorld` (`/Game/Prototype/Blueprints/LevelContent/InteractableObjects/Interactions/Activable/Utilities/BP_TeleportDestination.Teleport Position` _associated_teleport_destination))) false false))
    (:`Is Not Valid`
      (`KismetSystemLibrary.PrintString` "Teleport Destination not set"))))

(fn `UserConstructionScript`
  (`parent.UserConstructionScript`))