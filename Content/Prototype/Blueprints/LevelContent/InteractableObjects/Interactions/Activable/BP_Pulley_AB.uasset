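; Activable pulley object that moves its static mesh from a starting position to a destination once opened.
; Activate sets IsOpen and calls the parent logic, or clears the flag on a repeat call if the object is deactivable.
; While open, Tick keeps playing a timeline that lerps the mesh's world location between the two position components.
; Closing neither stops nor reverses the timeline.
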(event `self.ReceiveTick`
  (params (DeltaSeconds :type "Float (single-precision)"))
  (if (`self.Is Open`)
    (bind (_direction _newtrack_0) (`Timeline|Timeline` :`NewTime` DeltaSeconds)
      (:`Update`
        (`SceneComponent.K2_SetWorldLocation` (`self.StaticMesh`) (`KismetMathLibrary.VLerp` (`SceneComponent.K2_GetComponentLocation` (`self.Starting Position`)) (`SceneComponent.K2_GetComponentLocation` (`self.Destination Position`)) _newtrack_0) false false)))))

(fn `Activate`
  (bind _is_open (`self.Is Open`))
  (if _is_open
    (if (`self.Is Deactivable`)
      (set `self.Is Open` (not _is_open)))
    (else
      (set `self.Is Open` true)
      (`parent.Activate`))))

(fn `UserConstructionScript`
  (`parent.UserConstructionScript`))