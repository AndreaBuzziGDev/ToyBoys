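; Activable sliding door that opens when activated and can close again only if flagged as deactivable.
; Activate sets the open state and plays the matching sound at the door, calling the parent Activate only when opening.
; Tick plays or reverses a timeline from that state, whose alpha lerps the door cube's world location between closed and open marker components.
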(event `self.ReceiveTick`
  (params (DeltaSeconds :type "Float (single-precision)"))
  (if (`self.Is Open`)
    (bind (_direction _door_opening) (`Timeline|Timeline - Open Door (Rename Slide Open)` :`NewTime` DeltaSeconds :!label _label)
      (:`Update`
        (`SceneComponent.K2_SetWorldLocation` (`self.Cube`) (`KismetMathLibrary.VLerp` (`SceneComponent.K2_GetComponentLocation` (`self.Closed Door Position`)) (`SceneComponent.K2_GetComponentLocation` (`self.Open Door Position`)) _door_opening) false false)))
    (else
      (goto _label :!via `Reverse`))))

(fn `Activate`
  (bind _returnvalue (`self.K2_GetActorLocation`))
  (bind _is_open (`self.Is Open`))
  (if _is_open
    (if (`self.Is Deactivable`)
      (set `self.Is Open` (not _is_open))
      (`GameplayStatics.PlaySoundAtLocation` "/Game/Sounds/Environment/Interactions/Activables/Sliding_Door_Close.Sliding_Door_Close" _returnvalue (struct) 1.0 1.0 0.0 null null null null))
    (else
      (set `self.Is Open` true)
      (`parent.Activate`)
      (`GameplayStatics.PlaySoundAtLocation` "/Game/Sounds/Environment/Interactions/Activables/Sliding_Door_Open.Sliding_Door_Open" _returnvalue (struct) 1.0 1.0 0.0 null null null null))))

(fn `UserConstructionScript`)