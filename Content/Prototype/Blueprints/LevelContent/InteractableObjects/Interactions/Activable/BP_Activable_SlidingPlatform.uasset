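; An activable sliding platform that moves its cube to an open position once activated.
; Activate sets an open flag and calls the parent, and Tick then keeps playing a timeline while the flag is set.
; Each timeline update lerps the cube from its current world location toward the SlidOpenPosition marker by the DoorOpening value, without sweeping.
; This graph has no path back to closed.
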(event `self.ReceiveTick`
  (params (DeltaSeconds :type "Float (single-precision)"))
  (bind _cube (`self.Cube`))
  (if (`self.Is Open`)
    (bind (_direction _door_opening) (`Timeline|Timeline - Slide Open` :`NewTime` DeltaSeconds)
      (:`Update`
        (`SceneComponent.K2_SetWorldLocation` _cube (`KismetMathLibrary.VLerp` (`SceneComponent.K2_GetComponentLocation` _cube) (`SceneComponent.K2_GetComponentLocation` (`self.Slid Open Position`)) _door_opening) false false)))))

(fn `Activate`
  (set `self.Is Open` true)
  (`parent.Activate`))

(fn `UserConstructionScript`
  (`parent.UserConstructionScript`))