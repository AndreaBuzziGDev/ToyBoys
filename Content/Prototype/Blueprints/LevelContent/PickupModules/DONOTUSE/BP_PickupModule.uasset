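; BP_PickupModule is a pickup module actor that spins in the level and shows a prompt widget while the player overlaps it.
; A timeline, played from Tick, drives the root's yaw rotation.
; Box overlap with BP_ThirdPersonCharacter registers the module as its LastPickUpModule, creates WB_PickUpModules and sets IsPlayerColliding; leaving reverses all three.
; The pickup itself is not handled here, and the asset sits in a DONOTUSE folder.
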(event `self.ReceiveTick`
  (params (DeltaSeconds :type "Float (single-precision)"))
  (bind (_direction _rotate_constantly) (`Timeline|Timeline`)
    (:`Update`
      (`SceneComponent.K2_SetRelativeRotation` (`self.DefaultSceneRoot`) (`KismetMathLibrary.MakeRotator` 0.0 0.0 (* _rotate_constantly 360.0)) false false))))

(event `self.BoxCollision.OnComponentBeginOverlap`
  (params (OverlappedComponent :type "PrimitiveComponent Object Reference") (OtherActor :type "Actor Object Reference") (OtherComp :type "PrimitiveComponent Object Reference") (OtherBodyIndex :type Integer) (bFromSweep :type Boolean) (SweepResult :type "HitResult Structure (by ref)"))
  (`/Engine/EditorBlueprintResources/StandardMacros.IsValid` (`self.PickUpWdget`)
    (:`Is Not Valid`
      (bind _asbp_third_person_character (cast `/Game/Prototype/Blueprints/ThirdPersonCharacter/BP_ThirdPersonCharacter` OtherActor))
      (set `/Game/Prototype/Blueprints/ThirdPersonCharacter/BP_ThirdPersonCharacter.LastPickUpModule` self _asbp_third_person_character)
      (bind _returnvalue (`|CreateWidget` "/Game/Prototype/Blueprints/UI/PlayerHud/WB_PickUpModules.WB_PickUpModules_C" (`GameplayStatics.GetPlayerController` 0)))
      (bind _output_get (set `self.PickUpWdget` _returnvalue))
      (`UserWidget.AddToViewport` _output_get 0)
      (set `self.IsPlayerColliding` true))))

(event `self.BoxCollision.OnComponentEndOverlap`
  (params (OverlappedComponent :type "PrimitiveComponent Object Reference") (OtherActor :type "Actor Object Reference") (OtherComp :type "PrimitiveComponent Object Reference") (OtherBodyIndex :type Integer))
  (bind _asbp_third_person_character (cast `/Game/Prototype/Blueprints/ThirdPersonCharacter/BP_ThirdPersonCharacter` OtherActor))
  (set `/Game/Prototype/Blueprints/ThirdPersonCharacter/BP_ThirdPersonCharacter.LastPickUpModule` null _asbp_third_person_character)
  (`Widget.RemoveFromParent` (`self.PickUpWdget`))
  (set `self.PickUpWdget` null)
  (set `self.IsPlayerColliding` false))

(fn `UserConstructionScript`)