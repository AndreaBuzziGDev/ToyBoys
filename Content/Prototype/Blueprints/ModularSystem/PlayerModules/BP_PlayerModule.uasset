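; BP_PlayerModule is a prototype player module in a modular system, tied to an anatomic part and an input action.
; It listens for the Head, ArmLeft, ArmRight and Legs Enhanced Input actions starting.
; IsMatchingInputAction compares the triggered action's display name with the module's own InputAction, so the module reacts only to its assigned action.
; On a match it only prints its AnatomicPart, with no gameplay effect yet.
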(event `EnhancedInput|/Game/ThirdPerson/Input/Actions/Custom/IA_Head`
  (params (ActionValue :type Boolean) (ElapsedSeconds :type "Float (double-precision)") (TriggeredSeconds :type "Float (double-precision)") (InputAction :type "InputAction Object Reference" :default "/Game/ThirdPerson/Input/Actions/Custom/IA_Head.IA_Head"))
  (:`Started`
    (bind _ismatching (`self.IsMatchingInputAction` InputAction))
    (if _ismatching
      (`KismetSystemLibrary.PrintString` (`self.Anatomic Part`) :!label _label))))

(event `EnhancedInput|/Game/ThirdPerson/Input/Actions/Custom/IA_ArmLeft`
  (params (ActionValue :type Boolean) (ElapsedSeconds :type "Float (double-precision)") (TriggeredSeconds :type "Float (double-precision)") (InputAction :type "InputAction Object Reference" :default "/Game/ThirdPerson/Input/Actions/Custom/IA_ArmLeft.IA_ArmLeft"))
  (:`Started`
    (bind _ismatching (`self.IsMatchingInputAction` InputAction))
    (if _ismatching
      (goto _label))))

(event `EnhancedInput|/Game/ThirdPerson/Input/Actions/Custom/IA_ArmRight`
  (params (ActionValue :type Boolean) (ElapsedSeconds :type "Float (double-precision)") (TriggeredSeconds :type "Float (double-precision)") (InputAction :type "InputAction Object Reference" :default "/Game/ThirdPerson/Input/Actions/Custom/IA_ArmRight.IA_ArmRight"))
  (:`Started`
    (bind _ismatching (`self.IsMatchingInputAction` InputAction))
    (if _ismatching
      (goto _label))))

(event `EnhancedInput|/Game/ThirdPerson/Input/Actions/Custom/IA_Legs`
  (params (ActionValue :type Boolean) (ElapsedSeconds :type "Float (double-precision)") (TriggeredSeconds :type "Float (double-precision)") (InputAction :type "InputAction Object Reference" :default "/Game/ThirdPerson/Input/Actions/Custom/IA_Legs.IA_Legs"))
  (:`Started`
    (bind _ismatching (`self.IsMatchingInputAction` InputAction))
    (if _ismatching
      (goto _label))))

(fn `IsMatchingInputAction`
  (params (`Input to Compare` :type "InputAction Object Reference"))
  (returns (IsMatching :type Boolean))
  (return (`KismetStringLibrary.EqualEqual_StrStr` (`KismetSystemLibrary.GetDisplayName` (`self.Input Action`)) (`KismetSystemLibrary.GetDisplayName` (`local.Input to Compare`)))))