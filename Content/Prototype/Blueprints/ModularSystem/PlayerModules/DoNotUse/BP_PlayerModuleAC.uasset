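; Prototype base component for player body modules, kept in a DoNotUse folder.
; Head, left arm and right arm inputs call PerformAction only when the action's display name matches the module's InputAction.
; PerformAction just prints a generic message, and GetBurdenValue returns zero as a default.
; Legs and jump input events are empty, with a note that jumping is handled on the Third Person Character.
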(event `EnhancedInput|/Game/ThirdPerson/Input/Actions/Custom/IA_Head`
  (params (ActionValue :type Boolean) (ElapsedSeconds :type "Float (double-precision)") (TriggeredSeconds :type "Float (double-precision)") (InputAction :type "InputAction Object Reference" :default "/Game/ThirdPerson/Input/Actions/Custom/IA_Head.IA_Head"))
  (:`Started`
    (bind _ismatching (`self.IsMatchingInputAction` InputAction))
    (if _ismatching
      (`self.Perform Action` :!label _label))))

(event `EnhancedInput|/Game/ThirdPerson/Input/Actions/Custom/IA_ArmLeft`
  (params (ActionValue :type Boolean) (ElapsedSeconds :type "Float (double-precision)") (TriggeredSeconds :type "Float (double-precision)") (InputAction :type "InputAction Object Reference" :default "/Game/ThirdPerson/Input/Actions/Custom/IA_ArmLeft.IA_ArmLeft"))
  (:`Started`
    (bind _ismatching (`self.IsMatchingInputAction` InputAction))
    (if _ismatching
      (goto _label))))

(event `EnhancedInput|/Game/ThirdPerson/Input/Actions/Custom/IA_ArmRight`
  (params (ActionValue :type Boolean) (ElapsedSeconds :type "Float (double-precision)") (TriggeredSeconds :type "Float (double-precision)") (InputAction :type "InputAction Object Reference" :default "/Game/ThirdPerson/Input/Actions/Custom/IA_ArmRight.IA_ArmRight"))
  (:`Started`
    (bind _ismatching (`self.IsMatchingInputAction` InputAction))
    (if _ismatching
      (goto _label))))

(event `EnhancedInput|/Game/ThirdPerson/Input/Actions/Custom/IA_Legs`
  (params (ActionValue :type Boolean) (ElapsedSeconds :type "Float (double-precision)") (TriggeredSeconds :type "Float (double-precision)") (InputAction :type "InputAction Object Reference" :default "/Game/ThirdPerson/Input/Actions/Custom/IA_Legs.IA_Legs"))
  ;[1 1 1] Jump Action handled directly on Third Person Character
  ;;[1 1 1] TODO: UNUSED
)

(event `EnhancedInput|/Game/ThirdPerson/Input/Actions/IA_Jump`
  (params (ActionValue :type Boolean) (ElapsedSeconds :type "Float (double-precision)") (TriggeredSeconds :type "Float (double-precision)") (InputAction :type "InputAction Object Reference" :default "/Game/ThirdPerson/Input/Actions/IA_Jump.IA_Jump"))
  ;[1 1 1] Jump Action handled directly on Third Person Character
)

(event `/Game/Prototype/Blueprints/ModularSystem/PlayerModules/BI_ModuleActor.Perform Action`
  (`KismetSystemLibrary.PrintString` "Perform Action - GENERIC"))

(fn `Get Burden Value`
  (returns (Value :type "Float (double-precision)"))
  (return 0.0))

(fn `IsMatchingInputAction`
  (params (`Input to Compare` :type "InputAction Object Reference"))
  (returns (IsMatching :type Boolean))
  (return (`KismetStringLibrary.EqualEqual_StrStr` (`KismetSystemLibrary.GetDisplayName` (`self.Input Action`)) (`KismetSystemLibrary.GetDisplayName` `Input to Compare`))))