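; BP_ModuleLegs is the player's leg module in a modular character system, covering No Legs, Legs, Wheels and Springs variants.
; Per-variant maps supply burden, jump speed and walk speed, with Wheels unable to jump.
; InitSceneModule switches the character's BP_SceneLegs child actor to match.
; PerformAction only prints, as BP_ThirdPersonCharacter handles leg behavior, and GetMovementSpeedMultiplier sets MaxWalkSpeed directly, returning zero.
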(event `self.ReceiveTick`
  (params (DeltaSeconds :type "Float (single-precision)")))

(event `self.Perform Action`
  ;[1 1 1] NB: In Legs, this essentially does nothing. Leg Module is basically handled in the BP_ThirdPersonCharacter
  (switch `/Game/Prototype/Blueprints/ModularSystem/enums/E_Modules_Legs` (`self.Module`)
    (:`NewEnumerator0`
      (`KismetSystemLibrary.PrintString` "Regular Jump" :!label _label))
    (:`NewEnumerator1`
      (goto _label))
    (:`NewEnumerator2`
      (`KismetSystemLibrary.PrintString` "Wheels cannot jump"))
    (:`NewEnumerator3`
      (`KismetSystemLibrary.PrintString` "Super Jump!"))))

(event `/Game/Prototype/Blueprints/ModularSystem/PlayerModules/ActorComponentModules/BI_ModuleActor.Init Scene Module`
  (bind _asbp_scene_legs (cast `/Game/Prototype/Blueprints/ModularSystem/PlayerModules/ThirdPersonCharacterSceneModules/BP_SceneLegs` (`ChildActorComponent.ChildActor` (`/Game/Prototype/Blueprints/ThirdPersonCharacter/BP_ThirdPersonCharacter.BP_SceneLegs` (`self.Parent Character`)))))
  (`/Game/Prototype/Blueprints/ModularSystem/PlayerModules/ThirdPersonCharacterSceneModules/BP_SceneLegs.Switch Module` _asbp_scene_legs (`self.Module`)))

(fn `Get Burden Value`
  (returns (Value :type "Float (double-precision)"))
  (return (`BlueprintMapLibrary.Map_Find` (`self.Burden Mapping`) (`self.Module`))))

(fn `Get Movement Speed Multiplier`
  (returns (Result :type "Float (double-precision)"))
  (set `CharacterMovementComponent.MaxWalkSpeed` (`BlueprintMapLibrary.Map_Find` (`self.Movement Speed Mapping`) (`self.Module`)) (`Character.CharacterMovement` (`self.Parent Character`)))
  (return 0.0))

(fn `Is Jump Capable`
  (returns (Result :type Boolean) (`Jump Speed` :type "Float (double-precision)"))
  (bind _module (`self.Module`))
  (bind _value (`BlueprintMapLibrary.Map_Find` (`self.Jump Speed Mapping`) _module))
  (switch `/Game/Prototype/Blueprints/ModularSystem/enums/E_Modules_Legs` _module
    (:`NewEnumerator0`
      _)
    (:`NewEnumerator1`
      _)
    (:`NewEnumerator2`
      (return false _value))
    (:`NewEnumerator3`
      _))
  (return true _value))