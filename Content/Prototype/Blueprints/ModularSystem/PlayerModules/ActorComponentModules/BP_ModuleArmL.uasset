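; BP_ModuleArmL is the left-arm module component in the player's modular system.
; On init it switches the character's left-arm scene child actor to the current module, while its action only prints a debug message outside toy mode.
; Constant burden and activation cost are looked up per module from maps, with burden using the active or passive map according to the module's state and flags, defaulting to zero.
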(event `self.Perform Action`
  (if (not (`/Game/Prototype/Blueprints/ThirdPersonCharacter/BP_ThirdPersonCharacter.Is Toy Mode` (`self.Parent Character`)))
    (`KismetSystemLibrary.PrintString` "Perform Action - Module Arm Left")))

(event `/Game/Prototype/Blueprints/ModularSystem/PlayerModules/ThirdPersonCharacterSceneModules/DoNotUse/BI_ModuleActor.Init Scene Module`
  (bind _asbp_scene_arm_left (cast `/Game/Prototype/Blueprints/ModularSystem/PlayerModules/ThirdPersonCharacterSceneModules/BP_SceneArmLeft` (`ChildActorComponent.ChildActor` (`/Game/Prototype/Blueprints/ThirdPersonCharacter/BP_ThirdPersonCharacter.BP_SceneArmLeft` (`self.Parent Character`)))))
  (`/Game/Prototype/Blueprints/ModularSystem/PlayerModules/ThirdPersonCharacterSceneModules/BP_SceneArmLeft.Switch Module` _asbp_scene_arm_left (`self.Module`)))

(fn `Get Activation Cost`
  (returns (Value :type "Float (double-precision)"))
  (if (`self.Has Activation Cost`)
    (return (`BlueprintMapLibrary.Map_Find` (`self.Activation Costs`) (`self.Module`)))
    (else
      (return 0.0))))

(fn `Get Constant Burden`
  (returns (Value :type "Float (double-precision)"))
  (if (`self.Is Active`)
    (if (`self.Has Active Burden`)
      (return (`BlueprintMapLibrary.Map_Find` (`self.Burden Active Mapping`) (`self.Module`)))
      (else
        _))
    (elif (`self.Has Passive Burden`)
      (return (`BlueprintMapLibrary.Map_Find` (`self.Burden Passive Mapping`) (`self.Module`)))
      (else
        _)))
  (return 0.0))