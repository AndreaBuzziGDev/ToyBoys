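; BP_ModuleHead is the head module in the player's modular system.
; Its PerformAction event calls ToggleToyMode on the parent character.
; GetBurdenValue returns the module's burden by looking up its Module key in the MapBurdens map.
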(event `/Game/Prototype/Blueprints/ModularSystem/PlayerModules/ActorComponentModules/BI_ModuleActor.Perform Action`
  (`/Game/Prototype/Blueprints/ThirdPersonCharacter/BP_ThirdPersonCharacter.Toggle Toy Mode` (`self.Parent Character`)))

(fn `Get Burden Value`
  (returns (Value :type "Float (double-precision)"))
  (return (`BlueprintMapLibrary.Map_Find` (`self.Map Burdens`) (`self.Module`))))