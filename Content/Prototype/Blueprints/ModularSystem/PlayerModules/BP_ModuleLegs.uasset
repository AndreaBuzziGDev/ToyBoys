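; BP_ModuleLegs is the leg slot of a modular player system, with No Legs, Legs, Wheels and Springs variants.
; Map lookups keyed on the current Module supply burden, movement speed multiplier and jump speed.
; IsJumpCapable allows jumping for every variant except Wheels.
; PerformAction only prints debug text, as the author notes that leg behavior is basically handled in BP_ThirdPersonCharacter.
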(event `self.Perform Action`
  ;[1 1 1] NB: In Legs, this essentially does nothing. Leg Module is basically handled in the BP_ThirdPersonCharacter
  (switch `/Game/Prototype/Blueprints/ModularSystem/enums/E_Modules_Legs` (`self.Module`)
    (:`NewEnumerator0`
      (`KismetSystemLibrary.PrintString` "Regular Jump" :!label _label))
    (:`NewEnumerator1`
      (goto _label))
    (:`NewEnumerator2`
      (`KismetSystemLibrary.PrintString` "Wheels cannot jump"))
    (:`NewEnumerator3`
      (`KismetSystemLibrary.PrintString` "Super Jump!"))))

(fn `Get Burden Value`
  (returns (Value :type "Float (double-precision)"))
  (return (`BlueprintMapLibrary.Map_Find` (`self.Burden Mapping`) (`self.Module`))))

(fn `Get Movement Speed Multiplier`
  (returns (Result :type "Float (double-precision)"))
  (return (`BlueprintMapLibrary.Map_Find` (`self.Movement Speed Mapping`) (`self.Module`))))

(fn `Is Jump Capable`
  (returns (Result :type Boolean) (`Jump Speed` :type "Float (double-precision)"))
  (bind _module (`self.Module`))
  (bind _value (`BlueprintMapLibrary.Map_Find` (`self.Jump Speed Mapping`) _module))
  (switch `/Game/Prototype/Blueprints/ModularSystem/enums/E_Modules_Legs` _module
    (:`NewEnumerator0`
      _)
    (:`NewEnumerator1`
      _)
    (:`NewEnumerator2`
      (return false _value))
    (:`NewEnumerator3`
      _))
  (return true _value))