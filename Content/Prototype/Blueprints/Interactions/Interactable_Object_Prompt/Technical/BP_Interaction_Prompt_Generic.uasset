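; Generic interaction prompt actor that shows an on-screen prompt while the player character stands inside its detection box.
; Begin and end overlap events on the box filter for the third-person character and call a show/hide function.
; Showing creates a prompt widget for the first player controller, sets its module from the actor's prompt type and adds it to the viewport; hiding removes it and clears the reference.
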(event `self.Player Detection Box.OnComponentBeginOverlap`
  (params (OverlappedComponent :type "PrimitiveComponent Object Reference") (OtherActor :type "Actor Object Reference") (OtherComp :type "PrimitiveComponent Object Reference") (OtherBodyIndex :type Integer) (bFromSweep :type Boolean) (SweepResult :type "HitResult Structure (by ref)"))
  (cast `/Game/Prototype/Blueprints/ThirdPersonCharacter/BP_ThirdPersonCharacter` OtherActor)
  (`self.Handle Prompt Show` true))

(event `self.Player Detection Box.OnComponentEndOverlap`
  (params (OverlappedComponent :type "PrimitiveComponent Object Reference") (OtherActor :type "Actor Object Reference") (OtherComp :type "PrimitiveComponent Object Reference") (OtherBodyIndex :type Integer))
  (cast `/Game/Prototype/Blueprints/ThirdPersonCharacter/BP_ThirdPersonCharacter` OtherActor)
  (`self.Handle Prompt Show` false))

(fn `Handle Prompt Show`
  (params (`Is Prompt Visible` :type Boolean))
  (if `Is Prompt Visible`
    (bind _returnvalue (`|CreateWidget` "/Game/Prototype/Blueprints/UI/PlayerHud/WB_Prompt_Interaction_Module.WB_Prompt_Interaction_Module_C" (`GameplayStatics.GetPlayerController` 0)))
    (set `/Game/Prototype/Blueprints/UI/PlayerHud/WB_Prompt_Interaction_Module.Module` (`self.Prompt Type`) _returnvalue)
    (`UserWidget.AddToViewport` _returnvalue 0)
    (set `self.Prompt Blueprint` _returnvalue)
    (else
      (`Widget.RemoveFromParent` (`self.Prompt Blueprint`))
      (set `self.Prompt Blueprint` null))))

(fn `UserConstructionScript`)