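; Central game controller that handles input mode at start, game over, pause menu, player imprisonment and pickup respawning.
; Imprisonment, if the found patrol is chasing, resets the player's modules and teleports them to a prison chosen by FindClosestPrison, which compares player distance against stored location's vector length.
; Picked-up items are hidden with collision off; non-resource modules enter a timer map that Tick counts down before restoring them.
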(event `self.ReceiveBeginPlay`
  (`self.DoGameStart`))

(event `self.ReceiveTick`
  (params (DeltaSeconds :type "Float (single-precision)"))
  (`self.Manage Module Timers` DeltaSeconds))

(fn `Add Module To Respawn Queue`
  (params (`Picked Up Module` :type "/Game/Prototype/Blueprints/LevelContent/PickupModules/DONOTUSE/BP_PickupModule Object Reference"))
  (bind _defaultsceneroot (`/Game/Prototype/Blueprints/LevelContent/PickupModules/DONOTUSE/BP_PickupModule.DefaultSceneRoot` `Picked Up Module`))
  (cast `/Game/Prototype/Blueprints/LevelContent/PickupModules/DONOTUSE/BP_Pickup_Resources_Template` `Picked Up Module`
    (:`then`
      (`KismetSystemLibrary.PrintString` "Resources will not respawn"))
    (:`CastFailed`
      ;[1 1 1] Only actual Modules Respawn
      (`BlueprintMapLibrary.Map_Add` (`self.Module Respawn Timers`) `Picked Up Module` (`self.Default Module RT`))))
  (`SceneComponent.SetHiddenInGame` _defaultsceneroot true true)
  (`ActorComponent.SetComponentTickEnabled` _defaultsceneroot false)
  (`PrimitiveComponent.SetCollisionEnabled` (`/Game/Prototype/Blueprints/LevelContent/PickupModules/DONOTUSE/BP_PickupModule.BoxCollision` `Picked Up Module`) "NoCollision"))

(fn `DoGameOver`
  (bind _returnvalue (`GameplayStatics.GetPlayerController` 0))
  (bind _returnvalue_2 (`|CreateWidget` "/Game/Prototype/Blueprints/UI/MenuGameOver/WB_Menu_GameOver.WB_Menu_GameOver_C"))
  (`UserWidget.AddToViewport` _returnvalue_2 0)
  (`WidgetBlueprintLibrary.SetInputMode_UIOnlyEx` _returnvalue null)
  (set `PlayerController.bShowMouseCursor` true _returnvalue)
  (`GameplayStatics.SetGamePaused` true))

(fn `DoGameStart`
  (bind _returnvalue (`GameplayStatics.GetPlayerController` 0))
  (`WidgetBlueprintLibrary.SetInputMode_GameOnly` _returnvalue)
  (set `PlayerController.bShowMouseCursor` false _returnvalue))

(fn `Find Closest Prison`
  (params (Prisons :type "Array of /Game/Prototype/Blueprints/LevelContent/Prison/BP_PrisonLocation Object Reference") (Player :type "/Game/Prototype/Blueprints/ThirdPersonCharacter/BP_ThirdPersonCharacter Object Reference"))
  (returns (Output :type "/Game/Prototype/Blueprints/LevelContent/Prison/BP_PrisonLocation Object Reference"))
  (locals (`Min Distance` :type "Vector Structure") (`Closest Prison` :type "/Game/Prototype/Blueprints/LevelContent/Prison/BP_PrisonLocation Object Reference"))
  (for (_array_element _array_index) Prisons
    (if (== _array_index 0)
      (bind _returnvalue (`self.K2_GetActorLocation` _array_element))
      (set `local.Min Distance` _returnvalue)
      (set `local.Closest Prison` _array_element :!label _label)
      (elif (< (`KismetMathLibrary.Vector_Distance` _returnvalue (`self.K2_GetActorLocation` Player)) (`KismetMathLibrary.VSize` (`local.Min Distance`)))
        (set `local.Min Distance` _returnvalue)
        (goto _label))))
  (return (`local.Closest Prison`)))

(fn `HandlePause`
  (bind _returnvalue (`GameplayStatics.GetPlayerController` 0))
  (if (`GameplayStatics.IsGamePaused`)
    (`GameplayStatics.SetGamePaused` false)
    (`Widget.RemoveFromParent` (`self.Pause Menu Widget`))
    (`WidgetBlueprintLibrary.SetInputMode_GameOnly` _returnvalue)
    (set `PlayerController.bShowMouseCursor` false _returnvalue)
    (else
      (`GameplayStatics.SetGamePaused` true)
      (bind _returnvalue_2 (`|CreateWidget` "/Game/Prototype/Blueprints/UI/PauseMenu/PauseMenu.PauseMenu_C" _returnvalue))
      (bind _output_get (set `self.Pause Menu Widget` _returnvalue_2))
      (`UserWidget.AddToViewport` _output_get 0)
      (`WidgetBlueprintLibrary.SetInputMode_GameAndUIEx` _returnvalue _returnvalue_2)
      (set `PlayerController.bShowMouseCursor` true _returnvalue))))

(fn `Imprison Player`
  (bind _returnvalue (`GameplayStatics.GetActorOfClass` "/Game/AI/BP_TestPatrol.BP_TestPatrol_C"))
  (if (`/Game/AI/BP_TestPatrol.IsChasing` _returnvalue)
    (bind _returnvalue_2 (`GameplayStatics.GetActorOfClass` "/Game/Prototype/Blueprints/ThirdPersonCharacter/BP_ThirdPersonCharacter.BP_ThirdPersonCharacter_C"))
    (bind _output (`self.Find Closest Prison` (`self.Prisons`) _returnvalue_2))
    (`self.K2_SetActorLocation` _returnvalue_2 (`self.K2_GetActorLocation` _output) false false)
    (`/Game/Prototype/Blueprints/ThirdPersonCharacter/BP_ThirdPersonCharacter.Reset Modules` _returnvalue_2)
    (set `/Game/Prototype/Blueprints/ThirdPersonCharacter/BP_ThirdPersonCharacter.IsImprisoned` true _returnvalue_2)))

(fn `Manage Module Timers`
  (params (`Delta Seconds` :type "Float (double-precision)"))
  (bind _module_respawn_timers (`self.Module Respawn Timers`))
  (bind _keys (`BlueprintMapLibrary.Map_Keys` _module_respawn_timers))
  (for _array_element _keys
    (bind _returnvalue (- (`BlueprintMapLibrary.Map_Find` _module_respawn_timers _array_element) `Delta Seconds`))
    (`BlueprintMapLibrary.Map_Add` _module_respawn_timers _array_element _returnvalue)
    (if (>= 0.0 _returnvalue)
      (`self.Remove Module From Respawn Queue` _array_element))))

(fn `Remove Module From Respawn Queue`
  (params (`Respawned Module` :type "/Game/Prototype/Blueprints/LevelContent/PickupModules/DONOTUSE/BP_PickupModule Object Reference"))
  (bind _boxcollision (`/Game/Prototype/Blueprints/LevelContent/PickupModules/DONOTUSE/BP_PickupModule.BoxCollision` `Respawned Module`))
  (bind _rootcomponent (`Actor.RootComponent` `Respawned Module`))
  (`BlueprintMapLibrary.Map_Remove` (`self.Module Respawn Timers`) `Respawned Module`)
  (`SceneComponent.SetHiddenInGame` _rootcomponent false true)
  (`ActorComponent.SetComponentTickEnabled` _rootcomponent true)
  (`SceneComponent.SetHiddenInGame` _boxcollision true true)
  (`PrimitiveComponent.SetCollisionEnabled` _boxcollision "QueryOnly"))

(fn `UserConstructionScript`)