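; BP_Activable_MovingPlatform is an activatable prototype platform, with door-style naming, that slides its Cube toward the OpenDoorPosition marker.
; Activate sets IsOpen and calls the parent version, or clears the flag if already open and IsDeactivable.
; While IsOpen, Tick plays a timeline that lerps the Cube from its current location toward the marker without sweep.
; Deactivation has no return movement.
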(event `self.ReceiveTick`
  (params (DeltaSeconds :type "Float (single-precision)"))
  (bind _cube (`self.Cube`))
  (if (`self.Is Open`)
    (bind (_direction _door_opening) (`Timeline|Timeline - Open Door (Rename Slide Open)` :`NewTime` DeltaSeconds)
      (:`Update`
        (`SceneComponent.K2_SetWorldLocation` _cube (`KismetMathLibrary.VLerp` (`SceneComponent.K2_GetComponentLocation` _cube) (`SceneComponent.K2_GetComponentLocation` (`self.Open Door Position`)) _door_opening) false false)))))

(fn `Activate`
  (bind _is_open (`self.Is Open`))
  (if _is_open
    (if (`self.Is Deactivable`)
      (set `self.Is Open` (not _is_open)))
    (else
      (set `self.Is Open` true)
      (`parent.Activate`))))

(fn `UserConstructionScript`)