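; BP_GameControl is a game control Blueprint that handles the start and game-over states of play.
; On BeginPlay, DoGameStart switches to game-only input and hides the mouse cursor.
; DoGameOver adds the WB_Menu_GameOver widget to the viewport, switches to UI-only input, shows the cursor and pauses the game.
; Nothing in this Blueprint calls DoGameOver.
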(event `self.ReceiveBeginPlay`
  (`self.DoGameStart`))

(fn `DoGameOver`
  (bind _returnvalue (`GameplayStatics.GetPlayerController` 0))
  (bind _returnvalue_2 (`|CreateWidget` "/Game/Study_1/Blueprints/UI/Menu_GameOver/WB_Menu_GameOver.WB_Menu_GameOver_C"))
  (`UserWidget.AddToViewport` _returnvalue_2 0)
  (`WidgetBlueprintLibrary.SetInputMode_UIOnlyEx` _returnvalue null)
  (set `PlayerController.bShowMouseCursor` true _returnvalue)
  (`GameplayStatics.SetGamePaused` true))

(fn `DoGameStart`
  (bind _returnvalue (`GameplayStatics.GetPlayerController` 0))
  (`WidgetBlueprintLibrary.SetInputMode_GameOnly` _returnvalue)
  (set `PlayerController.bShowMouseCursor` false _returnvalue))

(fn `UserConstructionScript`)