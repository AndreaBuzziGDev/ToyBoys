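; Study Blueprint for an automatic double sliding door that opens while the first-person character stands in its trigger box.
; Box overlap begin and end events set an IsOpen flag, ignoring actors other than BP_FirstPersonCharacter.
; Tick lerps each door's world location toward its open or closed target component, using DeltaSeconds as alpha for an eased motion.
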(event `self.ReceiveTick`
  (params (DeltaSeconds :type "Float (single-precision)"))
  (bind _leftdoor (`self.LeftDoor`))
  (bind _rightdoor (`self.RightDoor`))
  (bind _leftdoor_2 (`self.LeftDoor`))
  (bind _rightdoor_2 (`self.RightDoor`))
  (if (`self.isOpen`)
    (`SceneComponent.K2_SetWorldLocation` _leftdoor (`KismetMathLibrary.VLerp` (`SceneComponent.K2_GetComponentLocation` _leftdoor) (`SceneComponent.K2_GetComponentLocation` (`self.Left Door Open Target Position`)) DeltaSeconds) false false)
    (`SceneComponent.K2_SetWorldLocation` _rightdoor (`KismetMathLibrary.VLerp` (`SceneComponent.K2_GetComponentLocation` _rightdoor) (`SceneComponent.K2_GetComponentLocation` (`self.Right Door Open Target Position`)) DeltaSeconds) false false)
    (else
      (`SceneComponent.K2_SetWorldLocation` _leftdoor_2 (`KismetMathLibrary.VLerp` (`SceneComponent.K2_GetComponentLocation` _leftdoor_2) (`SceneComponent.K2_GetComponentLocation` (`self.Left Door Closed Target Position`)) DeltaSeconds) false false)
      (`SceneComponent.K2_SetWorldLocation` _rightdoor_2 (`KismetMathLibrary.VLerp` (`SceneComponent.K2_GetComponentLocation` _rightdoor_2) (`SceneComponent.K2_GetComponentLocation` (`self.Right Door Closed Target Position`)) DeltaSeconds) false false))))

(event `self.Box Collision Activation.OnComponentBeginOverlap`
  (params (OverlappedComponent :type "PrimitiveComponent Object Reference") (OtherActor :type "Actor Object Reference") (OtherComp :type "PrimitiveComponent Object Reference") (OtherBodyIndex :type Integer) (bFromSweep :type Boolean) (SweepResult :type "HitResult Structure (by ref)"))
  (cast `/Game/Study_1/Blueprints/BP_FirstPersonCharacter` OtherActor)
  (set `self.isOpen` true))

(event `self.Box Collision Activation.OnComponentEndOverlap`
  (params (OverlappedComponent :type "PrimitiveComponent Object Reference") (OtherActor :type "Actor Object Reference") (OtherComp :type "PrimitiveComponent Object Reference") (OtherBodyIndex :type Integer))
  (cast `/Game/Study_1/Blueprints/BP_FirstPersonCharacter` OtherActor)
  (set `self.isOpen` false))

(fn `UserConstructionScript`)